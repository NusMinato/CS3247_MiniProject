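; BP_MineCart_Project5 is a lesson project mine cart actor that lights up while something is inside its box trigger and can be pushed along.
; Box overlap begin shows the cart's spot and point lights, and overlap end hides them.
; A SpeedUp event applies a large impulse along the cart base mesh's right vector and prints a debug message.
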(event `self.Box.OnComponentBeginOverlap`
  (params (OverlappedComponent :type "PrimitiveComponent Object Reference") (OtherActor :type "Actor Object Reference") (OtherComp :type "PrimitiveComponent Object Reference") (OtherBodyIndex :type Integer) (bFromSweep :type Boolean) (SweepResult :type "HitResult Structure (by ref)"))
  ;[1 1 1] Jump In
  (`SceneComponent.SetVisibility` (`self.Minecart_SpotLight`) true false)
  (`SceneComponent.SetVisibility` (`self.Minecart_PointLight`) true false)
  (`KismetSystemLibrary.Delay` 1.0))

(event `self.Box.OnComponentEndOverlap`
  (params (OverlappedComponent :type "PrimitiveComponent Object Reference") (OtherActor :type "Actor Object Reference") (OtherComp :type "PrimitiveComponent Object Reference") (OtherBodyIndex :type Integer))
  ;[1 1 1] Jump Out
  (`SceneComponent.SetVisibility` (`self.Minecart_PointLight`) false false)
  (`SceneComponent.SetVisibility` (`self.Minecart_SpotLight`) false false))

(event `SpeedUp`
  (bind _sm_minecart_base (`self.SM_MineCart_Base`))
  (`PrimitiveComponent.AddImpulse` _sm_minecart_base (* (`SceneComponent.GetRightVector` _sm_minecart_base) 1000000.0) "None" false)
  (`KismetSystemLibrary.PrintString` "Add Impulse"))

(fn `UserConstructionScript`)