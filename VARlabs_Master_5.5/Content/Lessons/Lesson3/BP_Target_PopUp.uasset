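; Pop-up target actor from Lesson 3 that moves vertically and is destroyed when interacted with.
; After a short delay on BeginPlay, the UpAndDown timeline drives a Z offset from the cached starting location.
; Interact prints a debug message, spawns a small neon explosion, destroys the actor and returns a fixed integer to the caller.
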(event `self.ReceiveBeginPlay`
  (set `self.Origin` (`self.K2_GetActorLocation`))
  (`KismetSystemLibrary.Delay` 2.0)
  (bind (_direction _data) (`Timeline|UpAndDown`)
    (:`Update`
      (`self.K2_SetActorLocation` (+ (`self.Origin`) (* _data (`KismetMathLibrary.MakeVector` 0.0 0.0 20.0)))))))

(fn `Interact`
  (returns (Score :type Integer))
  (`KismetSystemLibrary.PrintString` "Interact target" true true (struct :`G` 1.0 :`A` 1.0))
  (`GameplayStatics.SpawnEmitterAtLocation` "/Game/Effects/Particles/Explosion/P_NeonExplosion_Tiny.P_NeonExplosion_Tiny" (`self.K2_GetActorLocation`))
  (`self.K2_DestroyActor`)
  (return 5))

(fn `UserConstructionScript`)