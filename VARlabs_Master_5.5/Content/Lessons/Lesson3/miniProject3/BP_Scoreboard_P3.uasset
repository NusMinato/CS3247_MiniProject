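; BP_Scoreboard_P3 is a scoreboard actor for the Lesson 3 mini project that displays a score through a TextRender component.
; Its UpdateScore event takes a score, colors the text red when it is negative and green otherwise, then shows it as an integer.
; The actor does no work on BeginPlay, overlap or Tick, so the display changes only when UpdateScore is called.
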(event `UpdateScore`
  (params (Score :type Integer))
  (if (< Score 0)
    (`TextRenderComponent.SetTextRenderColor` (`self.TextRender`) (make `Color` 0 0 255 255))
    (else
      (`TextRenderComponent.SetTextRenderColor` (`self.TextRender`) (make `Color` 0 255 0 255))))
  (`TextRenderComponent.K2_SetText` (`self.TextRender`) (`KismetTextLibrary.Conv_IntToText` Score)))

(fn `UserConstructionScript`)