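; Barrel actor from a lesson mini-project that moves vertically on spawn and can be blown up through interaction.
; On BeginPlay, the Movement timeline's Height track offsets it along Z from its spawn location, and the barrel destroys itself when the timeline finishes.
; Interact plays a shot sound and a neon explosion at its location, destroys the actor and returns 1.
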(event `self.ReceiveBeginPlay`
  (set `self.Origin` (`self.K2_GetActorLocation`))
  (bind (_direction _height) (`Timeline|Movement`)
    (:`Update`
      (`self.K2_SetActorLocation` (+ (`self.Origin`) (* _height (`KismetMathLibrary.MakeVector` 0.0 0.0 160.0)))))
    (:`Finished`
      (`self.K2_DestroyActor`))))

(fn `Interact`
  (returns (Score :type Integer))
  (bind _returnvalue (`self.K2_GetActorLocation`))
  (`GameplayStatics.PlaySoundAtLocation` "/Game/Audio/SoundWaves/Effect/SW_Shot_2.SW_Shot_2" _returnvalue (struct) 1.0 1.0 0.0 null null null null)
  (`GameplayStatics.SpawnEmitterAtLocation` "/Game/Effects/Particles/Explosion/P_NeonExplosion.P_NeonExplosion" _returnvalue)
  (`self.K2_DestroyActor`)
  (return 1))

(fn `UserConstructionScript`)