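; BP_SwordSlash is a short-lived sword slash effect actor that plays a thud sound where it spawns.
; A timeline offsets it vertically from its starting location by a scaled Height curve while rotating it each update to face the player pawn.
; The actor destroys itself when the timeline finishes, and it has no active overlap or tick logic.
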(event `self.ReceiveBeginPlay`
  (bind (_startinglocation_x _startinglocation_y _startinglocation_z) (`KismetMathLibrary.BreakVector` (`self.StartingLocation`)))
  (bind _output_get (set `self.StartingLocation` (`self.K2_GetActorLocation`)))
  (`GameplayStatics.PlaySoundAtLocation` "/Game/Audio/SoundWaves/Effect/SW_Thud_3.SW_Thud_3" _output_get (struct) 1.0 1.0 0.0 null null null null)
  (bind (_direction _height) (`Timeline|Animation`)
    (:`Update`
      (`self.K2_SetActorLocationAndRotation` (`KismetMathLibrary.MakeVector` _startinglocation_x _startinglocation_y (+ _startinglocation_z (* _height 100.0))) (`KismetMathLibrary.FindLookAtRotation` (`self.K2_GetActorLocation`) (`self.K2_GetActorLocation` (`GameplayStatics.GetPlayerPawn` 0)))))
    (:`Finished`
      (`self.K2_DestroyActor`))))

(fn `UserConstructionScript`)