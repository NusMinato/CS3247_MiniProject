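; BP_SwordTrap is a sword projectile trap that flies in a straight line until it overlaps something or times out.
; Each Tick it moves along world negative X by Speed with a swept offset, not scaled by delta time.
; An overlap on the claymore mesh spawns a small neon explosion and laser sound, then destroys the actor, applying no damage.
; Otherwise, a BeginPlay delay destroys it after five seconds.
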(event `self.ReceiveBeginPlay`
  (`KismetSystemLibrary.Delay` 5.0)
  (`self.K2_DestroyActor`))

(event `self.ReceiveTick`
  (params (DeltaSeconds :type "Float (single-precision)"))
  (`self.K2_AddActorWorldOffset` (* (`self.Speed`) (`KismetMathLibrary.MakeVector` -1.0 0.0 0.0)) true))

(event `self.SM_Sword_Claymore.OnComponentBeginOverlap`
  (params (OverlappedComponent :type "PrimitiveComponent Object Reference") (OtherActor :type "Actor Object Reference") (OtherComp :type "PrimitiveComponent Object Reference") (OtherBodyIndex :type Integer) (bFromSweep :type Boolean) (SweepResult :type "HitResult Structure (by ref)"))
  (bind _returnvalue (`self.K2_GetActorLocation`))
  (`GameplayStatics.SpawnEmitterAtLocation` "/Game/Effects/Particles/Explosion/P_NeonExplosion_Tiny.P_NeonExplosion_Tiny" _returnvalue)
  (`GameplayStatics.PlaySoundAtLocation` "/Game/Audio/SoundWaves/Effect/SW_SmallLaser.SW_SmallLaser" _returnvalue (struct) 1.0 1.0 0.0 null null null null)
  (`self.K2_DestroyActor`))

(fn `UserConstructionScript`)