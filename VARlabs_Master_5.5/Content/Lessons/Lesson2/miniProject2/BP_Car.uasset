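; BP_Car is a lesson mini-project car actor that animates its wheels and explodes on a timer.
; Tick pitches four wheel conveyor meshes by a fixed step each frame, with opposite signs on alternating wheels, so the spin is frame-rate dependent.
; BeginPlay waits a few seconds, then spawns an asteroid explosion particle and sound at the actor's location and destroys itself.
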(event `self.ReceiveBeginPlay`
  (bind _returnvalue (`self.K2_GetActorLocation`))
  (`KismetSystemLibrary.Delay` 4.5)
  (`GameplayStatics.SpawnEmitterAtLocation` "/Game/Effects/Particles/Explosion/P_AsteroidExplosion.P_AsteroidExplosion" _returnvalue)
  (`GameplayStatics.PlaySoundAtLocation` "/Game/Audio/SoundWaves/Effect/SW_Explosion_3.SW_Explosion_3" _returnvalue (struct) 1.0 1.0 0.0 null null null null)
  (`self.K2_DestroyActor`))

(event `self.ReceiveTick`
  (params (DeltaSeconds :type "Float (single-precision)"))
  (`SceneComponent.K2_AddLocalRotation` (`self.SM_Wheel_Conveyor_A`) (`KismetMathLibrary.MakeRotator` 0.0 10.0) false false)
  (`SceneComponent.K2_AddLocalRotation` (`self.SM_Wheel_Conveyor_A1`) (`KismetMathLibrary.MakeRotator` 0.0 -10.0) false false)
  (`SceneComponent.K2_AddLocalRotation` (`self.SM_Wheel_Conveyor_A2`) (`KismetMathLibrary.MakeRotator` 0.0 10.0) false false)
  (`SceneComponent.K2_AddLocalRotation` (`self.SM_Wheel_Conveyor_A3`) (`KismetMathLibrary.MakeRotator` 0.0 -10.0) false false))

(fn `UserConstructionScript`)