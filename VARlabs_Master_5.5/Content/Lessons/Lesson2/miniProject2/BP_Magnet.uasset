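; BP_Magnet is a lesson mini-project magnet actor that pulls BP_Car actors toward itself while they overlap its Box.
; Every Tick it queries the Box for overlapping cars and offsets each one along the unit direction to the TargetPoint component, scaled by Speed.
; The move is swept, so collision can block it, and it is not scaled by delta time, so pull speed depends on frame rate.
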(event `self.ReceiveTick`
  (params (DeltaSeconds :type "Float (single-precision)"))
  ; Move towards magnet
  (for _array_element (`PrimitiveComponent.GetOverlappingActors` (`self.Box`) "/Game/Lessons/Lesson2/miniProject2/BP_Car.BP_Car_C")
    (if (not (== _array_element self))
      (`self.K2_AddActorWorldOffset` _array_element (* (`KismetMathLibrary.GetDirectionUnitVector` (`self.K2_GetActorLocation` _array_element) (`SceneComponent.K2_GetComponentLocation` (`self.TargetPoint`))) (`self.Speed`)) true false))))

(fn `UserConstructionScript`)