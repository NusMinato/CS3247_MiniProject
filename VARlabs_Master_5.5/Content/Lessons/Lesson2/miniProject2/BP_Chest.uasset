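; Lesson chest actor that opens when something overlaps its Box trigger.
; The overlap sets IsOpen and plays a timeline that rotates ChestLid around roll, then plays a chime at the chest when finished.
; While open, Tick lifts the TextRender by a fixed step each frame until a short Delay sets IsStop, so the rise distance depends on frame rate.
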(event `self.ReceiveBeginPlay`)

(event `self.ReceiveTick`
  (params (DeltaSeconds :type "Float (single-precision)"))
  (if (and (`self.IsOpen`) (not (`self.IsStop`)))
    (`SceneComponent.K2_AddWorldOffset` (`self.TextRender`) (0.0 0.0 6.0) false false)
    (`KismetSystemLibrary.Delay` 0.6)
    (set `self.IsStop` true)))

(event `self.Box.OnComponentBeginOverlap`
  (params (OverlappedComponent :type "PrimitiveComponent Object Reference") (OtherActor :type "Actor Object Reference") (OtherComp :type "PrimitiveComponent Object Reference") (OtherBodyIndex :type Integer) (bFromSweep :type Boolean) (SweepResult :type "HitResult Structure (by ref)"))
  (set `self.IsOpen` true)
  (bind (_direction _lid_degree) (`Timeline|时间轴`)
    (:`Update`
      (`SceneComponent.K2_SetRelativeRotation` (`self.ChestLid`) (`KismetMathLibrary.MakeRotator` _lid_degree) false false))
    (:`Finished`
      (`GameplayStatics.PlaySoundAtLocation` "/Game/Audio/SoundWaves/Effect/SW_Chime_2.SW_Chime_2" (`self.K2_GetActorLocation`) (struct) 1.0 1.0 0.0 null null null null))))

(fn `UserConstructionScript`)